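; CubeBP is a test actor, in a moving boat test folder, that travels along a spline path once play begins.
; On BeginPlay it finds the SplinePathBP actor in the level and starts the MoveObject timeline, with play rate set from TimeToCompleteInSeconds.
; Each timeline update maps the MoveTrack alpha to a distance along the spline and sets the actor's world location and rotation to that point.
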(event `self.ReceiveBeginPlay`
  (bind _returnvalue (`GameplayStatics.GetActorOfClass` "/Game/1_Muff/MovingBoatTest/SplinePathBP.SplinePathBP_C"))
  (set `self.Spine REF` _returnvalue)
  (`self.Move Object`))

(event `Move Object`
  (bind _spline (`/Game/1_Muff/MovingBoatTest/SplinePathBP.Spline` (`self.Spine REF`)))
  (`TimelineComponent.SetPlayRate` (`self.Move Object T`) (/ 1.0 (`self.Time To Complete (in Seconds)`)))
  (bind (_direction _move_track) (`Timeline|Move Object T`)
    (:`Update`
      (bind _returnvalue (`KismetMathLibrary.Lerp` 0.0 (`SplineComponent.GetSplineLength` (`/Game/1_Muff/MovingBoatTest/SplinePathBP.Spline` (`self.Spine REF`))) _move_track))
      (`self.K2_SetActorTransform` (`KismetMathLibrary.MakeTransform` (`SplineComponent.GetLocationAtDistanceAlongSpline` _spline _returnvalue "World") (`SplineComponent.GetRotationAtDistanceAlongSpline` _spline _returnvalue "World"))))))

(fn `UserConstructionScript`)